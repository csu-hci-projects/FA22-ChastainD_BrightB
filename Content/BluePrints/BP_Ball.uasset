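; Player-controlled physics ball that rolls, jumps and collects coins, and adds the UI_1 widget on BeginPlay.
; Movement axes share one torque call, camera input yaws the spring arm, and StopBall overrides linear and angular velocity.
; Jump applies a vertical impulse, re-enabled by any hit.
; Coin overlaps increment the GM_BallGame count and destroy the coin; at CoinGoal, an overlap instead boosts PlayerHealth up to 100 and resets the count.
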(event `InputAxis|Forward/Backward`
  (params (AxisValue :type "Float (single-precision)"))
  ;[1 1 1] Movement
  ;;[1 1 1] Rolling Around (X/Y)
  (`PrimitiveComponent.AddTorqueInRadians` (`self.SM_Ball`) (`KismetMathLibrary.MakeVector` (* (`self.AccellerationFactor`) (stale `InputAxis|Left/Right` AxisValue)) (* AxisValue (`self.AccellerationFactor`))) "None" true :!label _label))

(event `InputAction|StopBall`
  (params (Key :type "Key Structure"))
  ;[1 1 1] Movement
  ;;[1 1 1] When 0 is pressed, Stop all ball movement
  (:`Pressed`
    (`PrimitiveComponent.SetAllPhysicsLinearVelocity` (`self.SM_Ball`) (`KismetMathLibrary.Conv_IntToVector` (`self.StopPhysics`)) false)
    (`PrimitiveComponent.SetAllPhysicsAngularVelocityInRadians` (`self.SM_Ball`) (`KismetMathLibrary.Conv_IntToVector` (`self.StopPhysics`)) false)))

(event `InputAxis|Left/Right`
  (params (AxisValue :type "Float (single-precision)"))
  ;[1 1 1] Movement
  ;;[1 1 1] Rolling Around (X/Y)
  (goto _label))

(event `InputAxis|Camera Left/Right`
  (params (AxisValue :type "Float (single-precision)"))
  ;[1 1 1] Movement
  ;;[1 1 1] Camera Rotation
  (`SceneComponent.K2_AddLocalRotation` (`self.SpringArm`) (`KismetMathLibrary.MakeRotator` 0.0 0.0 (* AxisValue (`self.CameraAcceleration`))) false false))

(event `InputAction|Jump`
  (params (Key :type "Key Structure"))
  ;[1 1 1] Movement
  ;;[1 1 1] Jump (Z) and Play Sound
  (:`Pressed`
    (if (`self.CanJump`)
      (`PrimitiveComponent.AddImpulse` (`self.SM_Ball`) (`KismetMathLibrary.MakeVector` 0.0 0.0 (`self.Impulse`)) "None" true)
      (set `self.CanJump` false)
      (`GameplayStatics.PlaySound2D` "/Engine/VREditor/Sounds/UI/Laser_Push.Laser_Push" 1.0 1.0 0.0 null null))))

(event `self.ReceiveHit`
  (params (MyComp :type "PrimitiveComponent Object Reference") (Other :type "Actor Object Reference") (OtherComp :type "PrimitiveComponent Object Reference") (bSelfMoved :type Boolean) (HitLocation :type "Vector Structure") (HitNormal :type "Vector Structure") (NormalImpulse :type "Vector Structure") (Hit :type "HitResult Structure (by ref)"))
  ;[1 1 1] Movement
  ;;[1 1 1] If on ground, set CanJump to True. If CanJump is False play sound on jump.
  (if (not (`self.CanJump`))
    (`GameplayStatics.PlaySound2D` "/Engine/VREditor/Sounds/UI/Laser_Pull.Laser_Pull" 1.0 1.0 0.0 null null))
  (set `self.CanJump` true))

(event `self.ReceiveBeginPlay`
  ;[1 1 1] Game Progress
  ;;[1 1 1] UI
  (bind _returnvalue (`|CreateWidget` "/Game/BluePrints/UI/UI_1.UI_1_C"))
  (`UserWidget.AddToViewport` _returnvalue 0))

(event `self.ReceiveActorBeginOverlap`
  (params (OtherActor :type "Actor Object Reference"))
  ;[1 1 1] Game Progress
  ;;[1 1 1] Pick Up Coin / Play Sound / Add to Coin Count / Destroy Coin... After 5 coins have been collected, add 25 to PlayerHealth (or if >75 set back to 100) and set CoinCount to 0.
  (bind _ascoin (cast `/Game/BluePrints/Coin` OtherActor))
  (if (>= (`/Game/BluePrints/GM_BallGame.CoinCount` (stale _asgm_ball_game)) (`self.CoinGoal`))
    (`GameplayStatics.PlaySound2D` "/Game/Content/SuperGrid/TutorialLevel/SoundEffects/PingBing.PingBing" 1.0 1.0 0.0 null null)
    (bind _playerhealth (`/Game/BluePrints/GM_BallGame.PlayerHealth` (stale _asgm_ball_game)))
    (if (>= _playerhealth 75)
      (set `/Game/BluePrints/GM_BallGame.PlayerHealth` 100 (stale _asgm_ball_game))
      (set `/Game/BluePrints/GM_BallGame.CoinCount` 0 (stale _asgm_ball_game))
      (else
        (set `/Game/BluePrints/GM_BallGame.PlayerHealth` (+ _playerhealth 25) (stale _asgm_ball_game))
        (set `/Game/BluePrints/GM_BallGame.CoinCount` 0 (stale _asgm_ball_game))))
    (else
      (`GameplayStatics.PlaySound2D` "/Game/Content/SuperGrid/TutorialLevel/SoundEffects/MechClank.MechClank" 1.0 1.0 0.0 null null)
      (bind _asgm_ball_game (cast `/Game/BluePrints/GM_BallGame` (`GameplayStatics.GetGameMode`)))
      (set `/Game/BluePrints/GM_BallGame.CoinCount` (+ (`/Game/BluePrints/GM_BallGame.CoinCount` _asgm_ball_game) 1) _asgm_ball_game)
      (`self.K2_DestroyActor` _ascoin))))

(fn `Get_BP_Ball`
  (returns (self :type "Self Object Reference"))
  (return (`self.Self_0`)))

(fn `GetCamera`
  (returns (Camera :type "CameraComponent Object Reference"))
  (return (`self.Camera`)))

(fn `UserConstructionScript`)